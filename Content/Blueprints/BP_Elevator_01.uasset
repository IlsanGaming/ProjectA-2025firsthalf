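; Elevator actor that lifts its Cube platform along Z when F is pressed inside its trigger box.
; Any overlap with the Box enables player 0 input and shows the prompt Widget, and ending overlap reverses both.
; F plays a 2D sound, hides the widget and plays a Timeline that scales MoveLength into the Cube's relative location.
; The Timeline only plays forward, with no return trip.
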(event OnComponentBeginOverlap(Box)
  (params (OverlappedComponent :type Primitive%20Component%20Object%20Reference) (OtherActor :type Actor%20Object%20Reference) (OtherComp :type Primitive%20Component%20Object%20Reference) (OtherBodyIndex :type Integer) (bFromSweep :type Boolean) (SweepResult :type Hit%20Result%20Structure%20%28by%20ref%29))
  (Input|EnableInput (Game|GetPlayerController 0))
  (Rendering|SetVisibility (Variables|Default|GetWidget) true false))

(event OnComponentEndOverlap(Box)
  (params (OverlappedComponent :type Primitive%20Component%20Object%20Reference) (OtherActor :type Actor%20Object%20Reference) (OtherComp :type Primitive%20Component%20Object%20Reference) (OtherBodyIndex :type Integer))
  (Input|DisableInput (Game|GetPlayerController 0))
  (Rendering|SetVisibility (Variables|Default|GetWidget) false false))

(event Input|KeyboardEvents|F
  (params (Key :type Key%20Structure :default "None"))
  (:Pressed
    (Audio|PlaySound2D "/Game/Sounds/Elevator_01.Elevator_01" 1.0 1.0 0.0 0 0)
    (Rendering|SetVisibility (Variables|Default|GetWidget) false false)
    (bind _newtrack_0 (Timeline|Timeline Play)
      (:Update
        (Transformation|SetRelativeLocation (Variables|Default|GetCube) (* _newtrack_0 (Math|Vector|MakeVector 0.0 0.0 (Variables|Default|GetMoveLength))) false false)))))

(fn ConstructionScript)