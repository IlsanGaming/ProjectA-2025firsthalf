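; BP_Teleporter_02 is a teleporter that the player unlocks by pressing F, with no teleport logic in this graph.
; Overlapping the box enables input and shows a widget prompt, and leaving it disables input and hides the widget.
; The first press passes a DoOnce that hides the widget, swaps the active Niagara effects and plays an unlock sound.
; The overlap events still toggle the widget after unlocking.
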(event OnComponentBeginOverlap(Box)
  (params (OverlappedComponent :type Primitive%20Component%20Object%20Reference) (OtherActor :type Actor%20Object%20Reference) (OtherComp :type Primitive%20Component%20Object%20Reference) (OtherBodyIndex :type Integer) (bFromSweep :type Boolean) (SweepResult :type Hit%20Result%20Structure%20%28by%20ref%29))
  (Input|EnableInput (Game|GetPlayerController 0))
  (Rendering|SetVisibility (Variables|Default|GetWidget) true false))

(event OnComponentEndOverlap(Box)
  (params (OverlappedComponent :type Primitive%20Component%20Object%20Reference) (OtherActor :type Actor%20Object%20Reference) (OtherComp :type Primitive%20Component%20Object%20Reference) (OtherBodyIndex :type Integer))
  (Input|DisableInput (Game|GetPlayerController 0) 0)
  (Rendering|SetVisibility (Variables|Default|GetWidget) false false))

(event Input|KeyboardEvents|F
  (params (Key :type Key%20Structure))
  (:Pressed
    (Utilities|FlowControl|DoOnce false
      (:Completed
        (Rendering|SetVisibility (Variables|Default|GetWidget) false false)
        (Components|Activation|Deactivate (Variables|Default|GetNS_LtBoxSphere_Opened_Rare))
        (Components|Activation|Activate (Variables|Default|GetNS_LtBoxSphere_Opened_Rare2) false)
        (Audio|PlaySound2D "/Game/Sounds/TeleportUnlock_02.TeleportUnlock_02" 1.0 1.0 0.0 0 0)))))

(fn ConstructionScript)