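; BP_Pickup_01 is a pickup actor with a mesh and a text label that reacts to any overlap with its Box.
; Overlap toggles mesh and text visibility, waits two seconds, toggles the text again, then destroys the actor.
; Every tick, the text's relative yaw is set opposite the player camera's, billboarding it without pitch or roll.
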(event OnComponentBeginOverlap(Box)
  (params (OverlappedComponent :type Primitive%20Component%20Object%20Reference) (OtherActor :type Actor%20Object%20Reference) (OtherComp :type Primitive%20Component%20Object%20Reference) (OtherBodyIndex :type Integer) (bFromSweep :type Boolean) (SweepResult :type Hit%20Result%20Structure%20%28by%20ref%29))
  (Rendering|ToggleVisibility (Variables|Default|GetStaticMesh) false)
  (Rendering|ToggleVisibility (Variables|Default|GetTextRender) false)
  (Utilities|FlowControl|Delay 2.0)
  (Rendering|ToggleVisibility (Variables|Default|GetTextRender) false)
  (Actor|DestroyActor))

(event EventTick
  (params (DeltaSeconds :type Float%20%28single-precision%29))
  (Transformation|SetRelativeRotation (Variables|Default|GetTextRender) (Math|Rotator|MakeRotator 0.0 0.0 (+ (.yaw (Transformation|GetActorRotation (Game|GetPlayerCameraManager 0))) 1.8e+02)) false false))

(fn ConstructionScript)