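; Openable treasure chest that the player unlocks once by pressing F within its trigger box.
; Box overlap enables input and shows a prompt widget; end overlap hides the widget and calls DisableInput.
; Pressing F turns off box collision, hides the prompt and, through a DoOnce, plays a sound and a lid-rotation Timeline.
; Timeline updates also swap closed-state Niagara effects for opening ones, with the opened glow deactivated after a delay.
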(event OnComponentBeginOverlap(Box)
  (params (OverlappedComponent :type Primitive%20Component%20Object%20Reference) (OtherActor :type Actor%20Object%20Reference) (OtherComp :type Primitive%20Component%20Object%20Reference) (OtherBodyIndex :type Integer) (bFromSweep :type Boolean) (SweepResult :type Hit%20Result%20Structure%20%28by%20ref%29))
  (Input|EnableInput (Game|GetPlayerController 0))
  (Rendering|SetVisibility (Variables|Default|GetWidget) true false))

(event OnComponentEndOverlap(Box)
  (params (OverlappedComponent :type Primitive%20Component%20Object%20Reference) (OtherActor :type Actor%20Object%20Reference) (OtherComp :type Primitive%20Component%20Object%20Reference) (OtherBodyIndex :type Integer))
  (Input|DisableInput (Game|GetPlayerController 0) 0)
  (Rendering|SetVisibility (Variables|Default|GetWidget) false false))

(event Input|KeyboardEvents|F
  (params (Key :type Key%20Structure))
  (bind _upper (Variables|Default|GetUpper))
  (bind _ns_ltboxsquare_opened_rare (Variables|Default|GetNS_LtBoxSquare_Opened_Rare))
  (bind _returnvalue (Transformation|GetRelativeTransform _upper))
  (:Pressed
    (Collision|SetCollisionEnabled (Variables|Default|GetBox) "NoCollision")
    (Rendering|SetVisibility (Variables|Default|GetWidget) false false)
    (Utilities|FlowControl|DoOnce false
      (:Completed
        (Audio|PlaySoundatLocation "/Game/Sounds/TeleportUnlock_01.TeleportUnlock_01" (.location _returnvalue) "0, 0, 0" 1.0 1.0 0.0 0 0 0 0)
        (bind _newtrack_0 (Timeline|Timeline Play)
          (:Update
            (Transformation|SetRelativeTransform _upper (Math|Transform|MakeTransform (.location _returnvalue) (Math|Rotator|MakeRotator (.x _newtrack_0) 0.0 0.0) "1.000000,1.000000,1.000000") false false)
            (Components|Activation|Deactivate (Variables|Default|GetNS_LtBoxSquare_Closed_Rare))
            (Components|Activation|Activate _ns_ltboxsquare_opened_rare false)
            (Utilities|FlowControl|Delay 3.0)
            (Components|Activation|Deactivate _ns_ltboxsquare_opened_rare)))))))

(fn ConstructionScript)