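; BP_LightingEffectHandler is an actor that draws an electric arc effect between two offsets from its location, Origin and Target.
; BeginPlay creates a spline mesh with a dynamic material driven by arc noise scale and speed.
; Tick repositions the spline's endpoints to follow the actor.
; The audio setup is an empty stub, and the point light setup at Target exists but is never called.
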(event EventBeginPlay
  (bind _returnvalue (Transformation|GetActorLocation))
  (|CreateSpline_2)
  (|CreateAudio_2)
  (SplineMesh|SetStartandEnd (Variables|Default|GetSpline) (+ _returnvalue (Variables|Default|GetOrigin)) "0, 0, 0" (+ _returnvalue (Variables|Default|GetTarget)) "0, 0, 0" true :!class /Script/Engine.SplineMeshComponent))

(event EventTick
  (params (DeltaSeconds :type Float%20%28single-precision%29))
  (bind _returnvalue (Transformation|GetActorLocation))
  (SplineMesh|SetStartandEnd (Variables|Default|GetSpline) (+ _returnvalue (Variables|Default|GetOrigin)) "0, 0, 0" (+ _returnvalue (Variables|Default|GetTarget)) "0, 0, 0" true :!class /Script/Engine.SplineMeshComponent))

(fn ConstructionScript)