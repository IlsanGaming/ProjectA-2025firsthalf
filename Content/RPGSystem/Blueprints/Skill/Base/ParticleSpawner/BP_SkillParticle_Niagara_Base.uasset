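; Base actor for skill particle effects in the RPG system, playing a configurable Niagara system.
; On BeginPlay it assigns the Particle asset to its Niagara component and activates it, or destroys itself if no valid asset is set.
; The actor removes itself when the system finishes, or after DestroyTimer seconds if that value is positive.
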(event OnSystemFinished(Niagara)
  (params (PSystem :type Niagara%20Component%20Object%20Reference))
  ;[0.3698 0 0.007061] PLEASE ENABLE THE NIAGARA PLUGIN
  (Actor|DestroyActor))

(event EventBeginPlay
  (bind _particle (Variables|Default|GetParticle))
  (bind _niagara (Variables|Default|GetNiagara))
  (bind _destroytimer (Variables|Default|GetDestroyTimer))
  ;[0.3698 0 0.007061] PLEASE ENABLE THE NIAGARA PLUGIN
  (Utilities|IsValid _particle
    (:Is%20Valid
      (Class|NiagaraComponent|SetAsset _niagara _particle true)
      (Components|Activation|Activate _niagara true)
      (if (> _destroytimer 0.0)
        (Utilities|FlowControl|Delay _destroytimer)
        (Actor|DestroyActor)))
    (:Is%20Not%20Valid
      (Actor|DestroyActor))))

(fn ConstructionScript)