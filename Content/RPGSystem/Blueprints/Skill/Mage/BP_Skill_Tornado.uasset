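; Mage Tornado skill: a multi-hit AoE whirlwind that pulls valid targets toward its center.
; SkillStart attaches a vortex particle timed from the hit count and delay, runs the base skill start and sizes the overlap sphere from the skill's trace settings.
; Tick launches overlapping target characters inward, scaled by distance, until they are near the center allowing for mesh radius.
; OnAoeHitDone re-rolls damage slightly at or below the stored maximum.
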(event EventTick
  (params (DeltaSeconds :type Float%20%28single-precision%29))
  (bind _returnvalue (Transformation|GetActorLocation))
  (for _array_element (Collision|GetOverlappingActors (Variables|Default|GetSphere) "/Script/Engine.Actor" :!class /Script/Engine.PrimitiveComponent)
    (if (.Valid (CallFunction|IsValidTarget (Variables|Default|GetSkillOwner) _array_element))
      (bind _ascharacter (Utilities|Casting|CastToCharacter (Components|GetOwner (.Target%20 (CallFunction|IsValidTarget (Variables|Default|GetSkillOwner) _array_element)))))
      (bind _radius (Class|BPIRPGSystem|GetMeshRadius(Message) _ascharacter))
      (if (> (- (Utilities|GetDistanceLocation (Transformation|GetActorLocation _ascharacter) _returnvalue) _radius) 1e+02)
        (Character|LaunchCharacter _ascharacter (* (Math|Vector|GetForwardVector (Math|Rotator|FindLookatRotation (Transformation|GetActorLocation _ascharacter) _returnvalue)) (* (Utilities|GetDistanceLocation (Transformation|GetActorLocation _ascharacter) _returnvalue) 0.3)) false false)))))

(event EventOnAoeHitDone
  (params (Targets :type Array%20of%20BPC%20RPG%20System%20Object%20References))
  (bind _maxdamage (Variables|Default|GetMaxDamage))
  ;[1 1 1] Comment
  (Utilities|Struct|SetmembersinS_Skill (Variables|Default|GetSkillInfo) (Math|Random|RandomFloatinRange (* _maxdamage 0.98) _maxdamage)))

(event EventSkillStart
  (bind _skillinfo (Variables|Default|GetSkillInfo))
  (bind (_attacktype _damage _damagepercent _fixeddamage _multihitcount _multihitdelay _statbonus _maxdistance _addrangedattackdistance _selectlocation _requirestarget _attach _asyncaoe _tracetype _attackrangeoverwriteai _tracesettings _boxtracesettings) (Utilities|Struct|BreakS_Skill _skillinfo))
  (Variables|Default|SetMaxDamage _damage)
  (CallFunction|SpawnParticles "/Game/RPGSystem/Particles/P_Wirbel.P_Wirbel" "0, 0, 0" (Transformation|GetActorLocation) "0, 0, 0" "2.000000,2.000000,1.400000" (- (* _multihitcount _multihitdelay) 1.8) false self)
  (CallFunction|BasicSkillStart)
  (Components|Sphere|SetSphereRadius (Variables|Default|GetSphere) (Utilities|Select :Index _tracetype :NewEnumerator0 (.Radius (Utilities|Struct|BreakS_SkillTraceSettings _tracesettings)) :NewEnumerator1 (.Length (Utilities|Struct|BreakS_SkillBoxTraceSettings _boxtracesettings))) true))

(fn ConstructionScript
  (|CallParentFunction))