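; Mage whirl skill that plays a vortex effect on itself and triggers an area-of-effect hit.
; On SkillStart it spawns the P_Wirbel particles attached to the skill actor, with a destroy timer derived from the skill's multi-hit count.
; After a short delay it calls HitAoe, whose logic is not defined in this Blueprint.
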(event EventSkillStart
  (CallFunction|SpawnParticles "/Game/RPGSystem/Particles/P_Wirbel.P_Wirbel" "0, 0, 0" (Transformation|GetActorLocation) "0, 0, 0" "1.200000,1.200000,1.200000" (* (- (.MultiHitCount (Utilities|Struct|BreakS_Skill (Variables|Default|GetSkillInfo))) 2) 0.4) true self)
  (Utilities|FlowControl|Delay 0.3)
  (CallFunction|HitAoe))

(fn ConstructionScript
  (|CallParentFunction))