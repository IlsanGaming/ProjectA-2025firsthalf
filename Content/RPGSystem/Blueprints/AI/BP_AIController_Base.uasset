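; Base RPG AI controller that runs BT_Enemy and manages target acquisition for enemies, companions and minions.
; Pawn sensing and damage events feed CheckTarget, which writes valid, unobstructed targets to the Blackboard, favoring closer ones.
; Masters and slaves share targets through RPGSystem dispatchers with randomized delays, unbinding once engaged and rebinding on new searches.
; Target search can pause for a duration or until a slave nears its master.
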(event OnSeePawn(PawnSensing)
  (params (Pawn :type Pawn%20Object%20Reference))
  ;[1 1 1] On See Pawn
  (bind (_success _reference) (Class|BPIRPGSystem|GetRPGSystem(Message) Pawn))
  (if _success
    (CallFunction|CheckTarget _reference)))

(event Custom|OnDamageTaken
  (params (Attacker :type BPC%20RPG%20System%20Object%20Reference) (Damage :type Float%20%28double-precision%29) (DamageTo :type E_HealthType%20Enum :default "NewEnumerator0") (Impulse :type S%20Impulse%20Structure) (IsSE :type Boolean))
  ;[1 1 1] OnDamageTaken
  (CallFunction|CheckTarget Attacker))

(event Custom|MasterNewTarget
  (params (NewTarget :type BPC%20RPG%20System%20Object%20Reference))
  (bind _returnvalue (Components|GetOwner NewTarget))
  (bind _self self)
  (bind _rpgsystem (Variables|Components|GetRPGSystem))
  (bind _rpgsystem_2 (Variables|Components|GetRPGSystem))
  (bind _returnvalue_2 (AI|GetBlackboard _self))
  (bind _slavemaster (Variables|/Game/RPGSystem/Blueprints/BPC_RPGSystem.BPC_RPGSystem_C|GetSlaveMaster _rpgsystem_2))
  ;[1 1 1] Slave New Target from Master
  (Utilities|FlowControl|Delay (Math|Random|RandomFloatinRange 0.2 1.2)) ; Do add some randomness
  (Utilities|IsValid NewTarget
    (:Is%20Valid
      (Utilities|IsValid _returnvalue_2
        (:Is%20Valid
          (if (!= (AI|Components|Blackboard|GetValueasObject _returnvalue_2 (Utilities|Name|MakeLiteralName "SlaveMaster")) NewTarget)
            (if (or (Variables|/Game/RPGSystem/Blueprints/BPC_RPGSystem.BPC_RPGSystem_C|GetIsCompanion _rpgsystem) (Variables|/Game/RPGSystem/Blueprints/BPC_RPGSystem.BPC_RPGSystem_C|GetIsMinion _rpgsystem))
              (if (not (ScalableFloat|GetValueasBool _returnvalue_2 (Utilities|Name|MakeLiteralName "HasTarget")))
                (AI|Components|Blackboard|SetValueasObject _returnvalue_2 (Utilities|Name|MakeLiteralName "Target") _returnvalue :!label _label)
                (AI|Components|Blackboard|SetValueasBool _returnvalue_2 (Utilities|Name|MakeLiteralName "HasTarget") true)
                (AI|Components|Blackboard|SetValueasVector _returnvalue_2 (Utilities|Name|MakeLiteralName "TargetLocation") (Transformation|GetActorLocation _returnvalue))
                (Utilities|IsValid _slavemaster
                  (:Is%20Valid
                    (EventDispatchers|UnbindEventfromOnSlaveMasterNewTarget _slavemaster (EventDispatchers|CreateEvent :!event Custom|MasterNewTarget)))))
              (else
                (goto _label)))))))))

(event Custom|OnMasterDeath
  (params (Attacker :type BPC%20RPG%20System%20Object%20Reference) (Impulse :type S%20Impulse%20Structure) (Victim :type BPC%20RPG%20System%20Object%20Reference))
  ;[1 1 1] OnMasterDeath
  (AI|Components|Blackboard|SetValueasObject (Variables|Components|GetBlackboardReference) (Utilities|Name|MakeLiteralName "SlaveMaster") 0)
  (AI|Components|Blackboard|SetValueasBool (Variables|Components|GetBlackboardReference) (Utilities|Name|MakeLiteralName "IsSlave") false))

(event Custom|SlaveNewTarget
  (params (NewParam :type BPC%20RPG%20System%20Object%20Reference))
  (bind _returnvalue (Components|GetOwner NewParam))
  (bind _self self)
  (bind _rpgsystem (Variables|Components|GetRPGSystem))
  (bind _returnvalue_2 (AI|GetBlackboard _self))
  ;[1 1 1] Master new target from Slave
  (Utilities|FlowControl|Delay (Math|Random|RandomFloatinRange 0.5 1.0)) ; Do add some randomness
  (Utilities|IsValid NewParam
    (:Is%20Valid
      (Utilities|IsValid _returnvalue_2
        (:Is%20Valid
          (Utilities|IsValid (AI|Components|Blackboard|GetValueasObject _returnvalue_2 (Utilities|Name|MakeLiteralName "Target"))
            (:Is%20Not%20Valid
              (if (!= NewParam (Variables|Components|GetRPGSystem))
                (AI|Components|Blackboard|SetValueasObject _returnvalue_2 (Utilities|Name|MakeLiteralName "Target") _returnvalue)
                (AI|Components|Blackboard|SetValueasBool _returnvalue_2 (Utilities|Name|MakeLiteralName "HasTarget") true)
                (AI|Components|Blackboard|SetValueasVector _returnvalue_2 (Utilities|Name|MakeLiteralName "TargetLocation") (Transformation|GetActorLocation _returnvalue))
                (Default|CallOnSlaveMasterNewTarget _rpgsystem NewParam)
                (Default|CallOnSlaveFollowMe _rpgsystem)
                (EventDispatchers|UnbindEventfromOnSlaveNewTarget (Variables|Components|GetRPGSystem) (EventDispatchers|CreateEvent :!event Custom|SlaveNewTarget))))))))))

(event Custom|OnMasterMovementSpeedChanged
  (params (Speed :type Float%20%28double-precision%29))
  (bind _returnvalue (Pawn|GetControlledPawn))
  ;[1 1 1] On Master Movementspeed changed | Companion/Minion
  (bind _speed (Class|BPIRPGSystem|GetMovementSpeed(Message) _returnvalue))
  (Class|BPIRPGSystem|SetMovementSpeed(Message) _returnvalue false (Math|Float|SelectFloat Speed _speed (> Speed _speed))))

(event EventSetIsMaster
  ;[1 1 1] Comment
  (Utilities|IsValid (Variables|Components|GetRPGSystem)
    (:Is%20Valid
      (EventDispatchers|BindEventtoOnSlaveNewTarget (Variables|Components|GetRPGSystem) (EventDispatchers|CreateEvent :!event Custom|SlaveNewTarget))
      (Variables|Default|SetIsMaster true))))

(event EventPossess
  (params (PossessedPawn :type Pawn%20Object%20Reference))
  (bind _self self)
  (bind _pawnsensing (Variables|Components|GetPawnSensing))
  (bind _returnvalue (AI|GetBlackboard _self))
  ;[1 1 1] On Possess
  (Utilities|FlowControl|Sequence
    (:then_0
      (AI|RunBehaviorTree "/Game/RPGSystem/Blueprints/AI/BT_Enemy.BT_Enemy")
      (Utilities|IsValid _returnvalue
        (:Is%20Valid
          (Variables|Components|SetBlackboardReference _returnvalue)
          (bind (_success _reference) (Class|BPIRPGSystem|GetRPGSystemAI(Message) PossessedPawn))
          (if _success
            (bind _output_get (Variables|Components|SetRPGSystem _reference))
            (EventDispatchers|BindEventtoOnDamageTaken _output_get (EventDispatchers|CreateEvent :!event Custom|OnDamageTaken))
            (Utilities|FlowControl|Sequence
              (:then_0
                (if (not (Utilities|Struct|BreakS_Monster (Variables|/Game/RPGSystem/Blueprints/BPC_RPGSystem_AI.BPC_RPGSystem_AI_C|GetEnemyInfo _output_get)))
                  (Variables|/Script/AIModule.PawnSensingComponent|SetbSeePawns _pawnsensing false)
                  (Components|Activation|Deactivate _pawnsensing)))
              (:then_1
                (AI|Components|Blackboard|SetValueasEnum (AI|GetBlackboard self) (Utilities|Name|MakeLiteralName "AIState") (Variables|/Game/RPGSystem/Blueprints/BPC_RPGSystem.BPC_RPGSystem_C|GetAI%20State (Variables|Components|GetRPGSystem)))))))))
    (:then_1
      (Utilities|FlowControl|Delay 0.25)
      (Variables|Default|SetCanFindTarget true))))

(event EventUnPossess
  (params (UnpossessedPawn :type Pawn%20Object%20Reference))
  ;[1 1 1] On Unpossess
  (Actor|Tick|SetActorTickEnabled false)
  (Actor|DestroyActor))

(event EventSetIsSlave
  (bind _rpgsystem (Variables|Components|GetRPGSystem))
  ;[1 1 1] SetIsSlave
  (bind (_success _reference) (Class|BPIRPGSystem|GetRPGSystem(Message) (AI|Components|Blackboard|GetValueasObject (AI|GetBlackboard self) (Utilities|Name|MakeLiteralName "SlaveMaster"))))
  (if _success
    (Variables|Default|SetIsSlave true)
    (EventDispatchers|BindEventtoOnSlaveMasterNewTarget _reference (EventDispatchers|CreateEvent :!event Custom|MasterNewTarget))
    (if (or (Variables|/Game/RPGSystem/Blueprints/BPC_RPGSystem.BPC_RPGSystem_C|GetIsCompanion _rpgsystem) (Variables|/Game/RPGSystem/Blueprints/BPC_RPGSystem.BPC_RPGSystem_C|GetIsMinion _rpgsystem))
      (EventDispatchers|BindEventtoOnMovementSpeedChanged _reference (EventDispatchers|CreateEvent :!event Custom|OnMasterMovementSpeedChanged))
      (else
        (EventDispatchers|BindEventtoOnDeath _reference (EventDispatchers|CreateEvent :!event Custom|OnMasterDeath))))))

(event EventChangeSightRadius
  (params (Radius :type Float%20%28double-precision%29))
  (bind _pawnsensing (Variables|Components|GetPawnSensing))
  (bind _pawnsensing_2 (Variables|Components|GetPawnSensing))
  ;[1 1 1] Change Sight Radius
  (if (> Radius 0.0)
    (Variables|/Script/AIModule.PawnSensingComponent|SetSightRadius _pawnsensing Radius)
    (Variables|/Script/AIModule.PawnSensingComponent|SetbSeePawns _pawnsensing true)
    (Components|Activation|Activate _pawnsensing false)
    (Class|PawnSensingComponent|SetSensingUpdatesEnabled _pawnsensing true)
    (else
      (Variables|/Script/AIModule.PawnSensingComponent|SetSightRadius (Variables|Components|GetPawnSensing) 0.0)
      (Variables|/Script/AIModule.PawnSensingComponent|SetbSeePawns _pawnsensing_2 false)
      (Class|PawnSensingComponent|SetSensingUpdatesEnabled _pawnsensing_2 false)
      (Components|Activation|Deactivate _pawnsensing_2))))

(event EventSearchNewTarget
  (bind _pawnsensing (Variables|Components|GetPawnSensing))
  ;[1 1 1] Search for new target and re-enabling the dispatchers
  (CallFunction|EnableDispatchers)
  (Class|PawnSensingComponent|SetSensingInterval _pawnsensing 0.01)
  (Class|PawnSensingComponent|SetSensingUpdatesEnabled _pawnsensing true)
  (Utilities|FlowControl|Delay 0.2)
  (Class|PawnSensingComponent|SetSensingInterval (Variables|Components|GetPawnSensing) (Math|Random|RandomFloatinRange 0.2 1.5)))

(event EventDisableTargetSearchforDuration
  (params (Duration :type Float%20%28double-precision%29))
  ;[1 1 1] Disable Target Search For Duration
  (Variables|Default|SetCanFindTarget false)
  (CallFunction|DisableDispatchers)
  (Utilities|FlowControl|RetriggerableDelay Duration)
  (Variables|Default|SetCanFindTarget true)
  (CallFunction|EnableDispatchers))

(event EventDisableTargetSearchUntilinRangeOfMaster
  (bind _returnvalue (Pawn|GetControlledPawn))
  (bind _rpgsystem (Variables|Components|GetRPGSystem))
  (bind _slavemaster (Variables|/Game/RPGSystem/Blueprints/BPC_RPGSystem.BPC_RPGSystem_C|GetSlaveMaster _rpgsystem))
  ;[1 1 1] Disable Target Search until in range of Master
  (if (Variables|Default|GetIsSlave)
    (Variables|Default|SetCanFindTarget false)
    (CallFunction|DisableDispatchers)
    (Utilities|FlowControl|Delay 0.2 :!label _label)
    (Utilities|IsValid _slavemaster
      (:Is%20Valid
        (Utilities|IsValid _returnvalue
          (:Is%20Valid
            (if (<= (CallFunction|GetDistanceXY (Transformation|GetActorLocation _returnvalue) (Transformation|GetActorLocation (Components|GetOwner _slavemaster))) 5e+02)
              _
              (else
                (goto _label))))
          (:Is%20Not%20Valid
            _)))
      (:Is%20Not%20Valid
        _))
    (Variables|Default|SetCanFindTarget true)
    (CallFunction|EnableDispatchers)))

(fn ConstructionScript)

(fn CheckTarget
  (params (Target :type BPC%20RPG%20System%20Object%20Reference))
  (bind _returnvalue (Components|GetOwner Target))
  (bind _returnvalue_2 (Pawn|GetControlledPawn))
  (bind _returnvalue_3 (Pawn|GetControlledPawn))
  (bind _self self)
  (bind _self_2 self)
  (bind _rpgsystem (Variables|Components|GetRPGSystem))
  (bind _returnvalue_4 (AI|GetBlackboard _self_2))
  (bind _returnvalue_5 (AI|GetBlackboard _self))
  (if (Variables|Default|GetCanFindTarget)
    (Utilities|IsValid Target
      (:Is%20Valid
        (Utilities|FlowControl|Sequence
          (:then_0
            (Utilities|IsValid _returnvalue_2
              (:Is%20Valid
                (if (ScalableFloat|GetValueasBool _returnvalue_5 (Utilities|Name|MakeLiteralName "HasTarget"))
                  (if (< (Math|Vector|VectorLength (- (Transformation|GetActorLocation) (Transformation|GetActorLocation (Components|GetOwner Target)))) (Math|Vector|VectorLength (- (Transformation|GetActorLocation _returnvalue_2) (AI|Components|Blackboard|GetValueasVector _returnvalue_5 (Utilities|Name|MakeLiteralName "TargetLocation")))))
                    (if (CallFunction|IsValidTargetAI (Variables|Components|GetRPGSystem) Target) :!label _label
                      (bind _returnvalue_6 (Collision|LineTraceForObjects (Transformation|GetActorLocation _returnvalue_3) (Transformation|GetActorLocation (Components|GetOwner Target)) (Utilities|Array|MakeArray "ObjectTypeQuery1" "ObjectTypeQuery2") false (Utilities|Array|MakeArray _returnvalue_3) "None"))
                      (if (not _returnvalue_6)
                        (AI|Components|Blackboard|SetValueasObject _returnvalue_4 (Utilities|Name|MakeLiteralName "Target") _returnvalue)
                        (AI|Components|Blackboard|SetValueasBool _returnvalue_4 (Utilities|Name|MakeLiteralName "HasTarget") true)
                        (AI|Components|Blackboard|SetValueasVector _returnvalue_4 (Utilities|Name|MakeLiteralName "TargetLocation") (Transformation|GetActorLocation _returnvalue))
                        (EventDispatchers|UnbindEventfromOnDamageTaken (Variables|Components|GetRPGSystem) (EventDispatchers|CreateEvent :!event Custom|OnDamageTaken))
                        (if (Variables|Default|GetIsMaster)
                          (Default|CallOnSlaveMasterNewTarget _rpgsystem Target)
                          (Default|CallOnSlaveFollowMe _rpgsystem)
                          (EventDispatchers|UnbindEventfromOnSlaveNewTarget (Variables|Components|GetRPGSystem) (EventDispatchers|CreateEvent :!event Custom|SlaveNewTarget))
                          (else
                            (if (Variables|Default|GetIsSlave)
                              (if (Utilities|IsValid (Variables|/Game/RPGSystem/Blueprints/BPC_RPGSystem.BPC_RPGSystem_C|GetSlaveMaster (Variables|Components|GetRPGSystem)))
                                (EventDispatchers|UnbindEventfromOnSlaveMasterNewTarget (Variables|/Game/RPGSystem/Blueprints/BPC_RPGSystem.BPC_RPGSystem_C|GetSlaveMaster (Variables|Components|GetRPGSystem)) (EventDispatchers|CreateEvent :!event Custom|MasterNewTarget))))
                            (bind (_success _reference) (Class|BPIRPGSystem|GetRPGSystem(Message) (AI|Components|Blackboard|GetValueasObject (AI|GetBlackboard self) (Utilities|Name|MakeLiteralName "SlaveMaster"))))
                            (if _success
                              (Default|CallOnSlaveNewTarget _reference Target)))))))
                  (else
                    (goto _label))))))
          (:then_1
            (Class|PawnSensingComponent|SetSensingInterval (Variables|Components|GetPawnSensing) (Math|Random|RandomFloatinRange 0.2 1.5))))))))

(fn EnableDispatchers
  (bind _rpgsystem (Variables|Components|GetRPGSystem))
  (bind _slavemaster (Variables|/Game/RPGSystem/Blueprints/BPC_RPGSystem.BPC_RPGSystem_C|GetSlaveMaster _rpgsystem))
  (EventDispatchers|BindEventtoOnDamageTaken (Variables|Components|GetRPGSystem) (EventDispatchers|CreateEvent :!event Custom|OnDamageTaken))
  (Utilities|FlowControl|Sequence
    (:then_0
      (if (Variables|Default|GetIsSlave)
        (Utilities|IsValid _slavemaster
          (:Is%20Valid
            (EventDispatchers|BindEventtoOnSlaveMasterNewTarget _slavemaster (EventDispatchers|CreateEvent :!event Custom|MasterNewTarget))))))
    (:then_1
      (if (Variables|Default|GetIsMaster)
        (EventDispatchers|BindEventtoOnSlaveNewTarget (Variables|Components|GetRPGSystem) (EventDispatchers|CreateEvent :!event Custom|SlaveNewTarget))))))

(fn DisableDispatchers
  (bind _rpgsystem (Variables|Components|GetRPGSystem))
  (bind _slavemaster (Variables|/Game/RPGSystem/Blueprints/BPC_RPGSystem.BPC_RPGSystem_C|GetSlaveMaster _rpgsystem))
  (EventDispatchers|UnbindEventfromOnDamageTaken (Variables|Components|GetRPGSystem) (EventDispatchers|CreateEvent :!event Custom|OnDamageTaken))
  (Utilities|FlowControl|Sequence
    (:then_0
      (if (Variables|Default|GetIsSlave)
        (Utilities|IsValid _slavemaster
          (:Is%20Valid
            (EventDispatchers|UnbindEventfromOnSlaveMasterNewTarget _slavemaster (EventDispatchers|CreateEvent :!event Custom|MasterNewTarget))))))
    (:then_1
      (if (Variables|Default|GetIsMaster)
        (EventDispatchers|UnbindEventfromOnSlaveNewTarget (Variables|Components|GetRPGSystem) (EventDispatchers|CreateEvent :!event Custom|SlaveNewTarget))))))