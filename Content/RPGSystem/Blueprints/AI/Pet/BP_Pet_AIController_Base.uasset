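; Base AI controller for pets that follow a master and target nearby item drops for looting.
; InitPet loads the pet's DT_Pet row to configure autoloot ranges and binds to the master's inventory events.
; A sphere on the pawn queues matching drops; the nearest feeds BT_Pet's blackboard, limited to one item type when inventory is full.
; Pet speed scales from the master's, rising while chasing a target.
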(event OnComponentBeginOverlap(Sphere)
  (params (OverlappedComponent :type Primitive%20Component%20Object%20Reference) (OtherActor :type Actor%20Object%20Reference) (OtherComp :type Primitive%20Component%20Object%20Reference) (OtherBodyIndex :type Integer) (bFromSweep :type Boolean) (SweepResult :type Hit%20Result%20Structure%20%28by%20ref%29))
  ;[1 1 1] Overlap with Items
  (CallFunction|CheckTarget OtherActor))

(event OnComponentEndOverlap(Sphere)
  (params (OverlappedComponent :type Primitive%20Component%20Object%20Reference) (OtherActor :type Actor%20Object%20Reference) (OtherComp :type Primitive%20Component%20Object%20Reference) (OtherBodyIndex :type Integer))
  ;[1 1 1] Overlap with Items
  (if (Variables|Default|GetPetMasterFull)
    (Utilities|Array|RemoveItem (Variables|Default|GetItemToLoot) OtherActor)))

(event Custom|PetMasterInventoryChanged
  (params (Index :type Integer))
  (bind (_success _index) (CallFunction|GetNearest))
  ;[1 1 1] PetMasterInventoryChanged
  (if (Variables|Default|GetPetMasterFull)
    (Utilities|IsValid (Variables|Default|GetTarget)
      (:Is%20Not%20Valid
        (Variables|Default|SetPetMasterFull false)
        (if (> (Utilities|Array|Length (Variables|Default|GetItemToLoot)) 0)
          (if _success
            (CallFunction|UpdateTarget (Utilities|Array|Get(acopy) (Variables|Default|GetItemToLoot) _index)))
          (else
            (CallFunction|UpdateTarget)))))))

(event Custom|PetMasterInventoryFull
  ;[1 1 1] InitPet
  (Variables|Default|SetPetMasterFull true)
  (CallFunction|UpdateTarget))

(event EventPossess
  (params (PossessedPawn :type Pawn%20Object%20Reference))
  ;[1 1 1] On Possess
  (AI|RunBehaviorTree "/Game/RPGSystem/Blueprints/AI/Pet/BT_Pet.BT_Pet")
  (Transformation|AttachComponentToComponent (Variables|Default|GetSphere) (Actor|GetComponentbyClass PossessedPawn "/Script/Engine.CapsuleComponent") "None" "SnapToTarget" "SnapToTarget" "KeepRelative" true))

(event EventUnPossess
  (params (UnpossessedPawn :type Pawn%20Object%20Reference))
  ;[1 1 1] On Unpossess
  (Actor|Tick|SetActorTickEnabled false)
  (Actor|DestroyActor))

(event EventInitPet
  (params (PetID :type Name :default "None") (PetMaster :type Actor%20Object%20Reference))
  (bind _self self)
  (bind _returnvalue (AI|GetBlackboard _self))
  ;[1 1 1] InitPet
  (Variables|Default|SetPetID PetID)
  (bind _output_get (Variables|Default|SetPetMaster PetMaster))
  (bind (_success _reference) (Class|BPIRPGSystem|GetRPGSystem(Message) _output_get))
  (if _success
    (Variables|Default|SetPetMasterRPGSystem _reference)
    (bind _speed (Class|BPIRPGSystem|GetMovementSpeed(Message) PetMaster))
    (Class|BPIRPGSystem|SetMovementSpeed(Message) (Pawn|GetControlledPawn) false (* _speed 1.1))
    (bind _returnvalue_2 (Utilities|GetDataTableRow "/Game/RPGSystem/Blueprints/Database/DT_Pet.DT_Pet" PetID)
      (:then
        (Variables|Default|SetPetInfo _returnvalue_2)
        (EventDispatchers|BindEventtoOnInventoryFull (Variables|Default|GetPetMasterRPGSystem) (delegate Custom|PetMasterInventoryFull))
        (EventDispatchers|BindEventtoOnInventoryChanged (Variables|Default|GetPetMasterRPGSystem) (delegate Custom|PetMasterInventoryChanged))
        (AI|Components|Blackboard|SetValueasFloat _returnvalue (Utilities|Name|MakeLiteralName "PickupRange") (Math|Float|SelectFloat (.PickupRange (Utilities|Struct|BreakS_Pet _returnvalue_2)) 0.0 (.Autoloot (Utilities|Struct|BreakS_Pet _returnvalue_2))))
        (AI|Components|Blackboard|SetValueasObject _returnvalue (Utilities|Name|MakeLiteralName "PetMaster") PetMaster)
        (Variables|Default|SetCanFindTarget true)
        (Components|Sphere|SetSphereRadius (Variables|Default|GetSphere) (Math|Float|SelectFloat (.SightRange (Utilities|Struct|BreakS_Pet _returnvalue_2)) 0.0 (.Autoloot (Utilities|Struct|BreakS_Pet _returnvalue_2))) true)
        (if (.Autoloot (Utilities|Struct|BreakS_Pet _returnvalue_2))
          (Components|Activation|Deactivate (Variables|Default|GetSphere))))
      (:RowNotFound
        (CallFunction|PrintMessage "ERROR: WRONG PETID" 2.0)
        (Actor|DestroyActor (Pawn|GetControlledPawn))))
    (else
      (Actor|DestroyActor (Pawn|GetControlledPawn)))))

(event EventPetGetNewTarget
  (bind (_success _index) (CallFunction|GetNearest))
  ;[1 1 1] Get new Target
  (Utilities|Array|RemoveItem (Variables|Default|GetItemToLoot) (Variables|Default|GetTarget))
  (Variables|Default|SetTarget 0)
  (if _success
    (CallFunction|UpdateTarget (Utilities|Array|Get(acopy) (Variables|Default|GetItemToLoot) _index))
    (else
      (CallFunction|UpdateTarget))))

(fn ConstructionScript)

(fn CheckTarget
  (params (Item :type Actor%20Object%20Reference))
  (bind _returnvalue (Transformation|GetActorLocation))
  (bind _petinfo (Variables|Default|GetPetInfo))
  (bind _itemtypetoloot (Utilities|Struct|BreakS_Pet _petinfo))
  (if (Variables|Default|GetCanFindTarget)
    (bind _asbp_item_base (Utilities|Casting|CastToBP_Item_Base Item))
    (if (and (or (<= (Utilities|Array|Length _itemtypetoloot) 0) (Utilities|Array|ContainsItem _itemtypetoloot (Variables|/Game/RPGSystem/Blueprints/Item/BP_Item_Base.BP_Item_Base_C|GetItemType _asbp_item_base))) (Variables|/Game/RPGSystem/Blueprints/Item/BP_Item_Base.BP_Item_Base_C|GetNewDrop _asbp_item_base))
      (Utilities|IsValid (Variables|Default|GetTarget)
        (:Is%20Valid
          (if (< (Math|Vector|VectorLength (- _returnvalue (Transformation|GetActorLocation Item))) (Math|Vector|VectorLength (- _returnvalue (Transformation|GetActorLocation (Variables|Default|GetTarget)))))
            (Utilities|Array|AddUnique (Variables|Default|GetItemToLoot) Item)
            (CallFunction|UpdateTarget Item :!label _label)
            (else
              (Utilities|Array|AddUnique (Variables|Default|GetItemToLoot) Item))))
        (:Is%20Not%20Valid
          (Utilities|Array|AddUnique (Variables|Default|GetItemToLoot) Item)
          (goto _label))))))

(fn GetNearest
  (for (_array_element _array_index) (Variables|Default|GetItemToLoot)
    (Utilities|IsValid _array_element
      (:Is%20Valid
        (bind _itemtype (Class|BPIItem|GetItemInfo(Message) _array_element))
        (if (Utilities|Enum|Equal(Enum) _itemtype "NewEnumerator26")
          (if (< (Math|Vector|VectorLength (- (Transformation|GetActorLocation _array_element) (Transformation|GetActorLocation))) (LocalVariables|GetVarNearest)) :!label _label
            (LocalVariables|SetVarNearest (Math|Vector|VectorLength (- (Transformation|GetActorLocation _array_element) (Transformation|GetActorLocation))))
            (LocalVariables|SetVarIndex _array_index))
          (elif (not (Variables|Default|GetPetMasterFull))
            (goto _label))))))
  (return (> (LocalVariables|GetVarIndex) -1) (LocalVariables|GetVarIndex)))

(fn UpdateTarget
  (params (Target :type Actor%20Object%20Reference))
  (bind _returnvalue (Utilities|Name|MakeLiteralName "TargetLocation"))
  (bind _self self)
  (bind _petmaster (Variables|Default|GetPetMaster))
  (bind _returnvalue_2 (AI|GetBlackboard _self))
  (Variables|Default|SetTarget Target)
  (AI|Components|Blackboard|SetValueasObject _returnvalue_2 (Utilities|Name|MakeLiteralName "Target") (Variables|Default|GetTarget))
  (AI|Components|Blackboard|SetValueasBool _returnvalue_2 (Utilities|Name|MakeLiteralName "HasTarget") true)
  (Utilities|IsValid (Variables|Default|GetTarget)
    (:Is%20Valid
      (AI|Components|Blackboard|SetValueasVector _returnvalue_2 _returnvalue (Transformation|GetActorLocation (Variables|Default|GetTarget)))
      (bind _speed (Class|BPIRPGSystem|GetMovementSpeed(Message) _petmaster))
      (Class|BPIRPGSystem|SetMovementSpeed(Message) (Pawn|GetControlledPawn) false (* _speed 1.4)))
    (:Is%20Not%20Valid
      (AI|Components|Blackboard|SetValueasVector _returnvalue_2 _returnvalue "0, 0, 0")
      (bind _speed_2 (Class|BPIRPGSystem|GetMovementSpeed(Message) _petmaster))
      (Class|BPIRPGSystem|SetMovementSpeed(Message) (Pawn|GetControlledPawn) false (* _speed_2 1.1)))))