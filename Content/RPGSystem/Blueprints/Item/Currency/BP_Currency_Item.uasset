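; Currency pickup item Blueprint in the RPG system that represents dropped coins in the world.
; On BeginPlay it runs the parent logic, then tints its particle system gold through a color parameter.
; When the item count exceeds a threshold, a weighted random roll can swap the static mesh to a medium coin.
; The construction script only calls the parent.
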(event EventBeginPlay
  (|CallParentFunction)
  (Effects|Components|ParticleSystem|SetColorParameter (Variables|Default|GetParticleSystem) "Color" "(R=1.000000,G=0.880000,B=0.000000,A=1.000000)")
  (if (> (.Count (Utilities|Struct|BreakS_Inventory (Variables|Default|GetItem))) 200)
    (if (Math|Random|RandomBoolwithWeight 0.65)
      (Components|StaticMesh|SetStaticMesh (Variables|Default|GetStaticMesh) "/Game/RPGSystem/Models/GoldCoin/Mesh/SM_Coin_Medium.SM_Coin_Medium"))))

(fn ConstructionScript
  (|CallParentFunction))