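; Base treasure actor for the RPG system that players open once to drop loot.
; It supplies tooltips, a custom-depth selection outline and a move-to point in front for range checks.
; Interact runs on authority, distance-checking tooltip commands, then plays the animation and increments global and per-player custom variables through the GameInstance.
; After a short delay, BPCDropSystem spawns drops using the player's level and drop/gold bonuses, and the open event fires.
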(event Custom|OpenTreasure
  ;[1 1 1] Open animation
  (Audio|Components|Audio|Play (Variables|Components|GetSkeletalMesh) false)
  (Rendering|SetRenderCustomDepth (Variables|Components|GetSkeletalMesh) false))

(event Custom|StartDrop
  (bind _player (Variables|Components|GetPlayer))
  (bind _droppoint (Variables|Components|GetDropPoint))
  (bind _returnvalue (Transformation|GetWorldTransform _droppoint))
  (bind _playerinfo (Variables|/Game/RPGSystem/Blueprints/BPC_RPGSystem.BPC_RPGSystem_C|GetPlayerInfo _player))
  (bind _stats (Utilities|Struct|BreakS_PlayerInfo _playerinfo))
  (bind (_cashgainrate _dropratebonus) (Utilities|Struct|BreakS_Stats _stats))
  ;[1 1 1] Start Drop
  (Default|StartDrop (Variables|Components|GetBPC_DropSystem) (Variables|/Game/RPGSystem/Blueprints/BPC_RPGSystem.BPC_RPGSystem_C|GetBaseLevel _player) _dropratebonus _cashgainrate (.location _returnvalue) (.rotation _returnvalue)))

(event EventBeginPlay
  ;[1 1 1] Add Skeletal Mesh Radius to InteractRange
  (Variables|Default|SetMinDistanceToInteract (+ (Variables|Default|GetMinDistanceToInteract) (.SphereRadius (Collision|GetComponentBounds (Variables|Components|GetSkeletalMesh)))))
  (if (Variables|Default|GetOpen)
    (Components|Animation|PlayAnimation (Variables|Components|GetSkeletalMesh) "/Game/RPGSystem/Models/Treasure/Animation/Treasure_Opening.Treasure_Opening" false)))

(event EventSelectInteractable
  (params (Selected :type Boolean))
  ;[1 1 1] Outline
  (Rendering|SetRenderCustomDepth (Variables|Components|GetSkeletalMesh) (and Selected (not (Variables|Default|GetOpen)))))

(event EventInteract
  (params (RPGSystem :type BPC%20RPG%20System%20Object%20Reference) (Command :type String))
  ;[1 1 1] Interact
  (Networking|SwitchHasAuthority
    (:Authority
      (if (not (Variables|Default|GetOpen))
        (if (Utilities|Enum|Equal(Enum) Command "FromTooltip")
          (if (< (- (Utilities|GetDistanceLocation (Transformation|GetActorLocation (Components|GetOwner RPGSystem)) (Transformation|GetActorLocation)) (+ (.SphereRadius (Collision|GetComponentBounds (Variables|Components|GetSkeletalMesh))) 45.0)) 5e+01)
            (Variables|Default|SetOpen true :!label _label)
            (bind _output_get (Variables|Components|SetPlayer RPGSystem))
            (CallFunction|OpenTreasure)
            (CallFunction|AddCustomVariablestoPlayer (Variables|/Game/RPGSystem/Blueprints/BPC_RPGSystem.BPC_RPGSystem_C|GetUniqueID _output_get))
            (Utilities|FlowControl|Delay 0.7)
            (CallFunction|StartDrop)
            (Default|CallOnOpenTreasure))
          (else
            (goto _label)))))))

(fn ConstructionScript)

(fn GetCustomVariables
  (LocalVariables|SetVarCustomVariables (Variables|Configuration|GetCustomVariables))
  (LocalVariables|SetVarCustomVariablesPrivate (Variables|Configuration|GetCustomVariablesPrivate))
  (for _array_element (Variables|Configuration|GetCustomVariablesTags)
    (Utilities|Array|Add (LocalVariables|GetVarCustomVariables) (GameplayTags|GetTagName _array_element)))
  (for _array_element_2 (Variables|Configuration|GetCustomVariablesTagsPrivate)
    (Utilities|Array|Add (LocalVariables|GetVarCustomVariablesPrivate) (GameplayTags|GetTagName _array_element_2)))
  (return (Utilities|Struct|MakeS_ArrayOf_FName (LocalVariables|GetVarCustomVariables)) (Utilities|Struct|MakeS_ArrayOf_FName (LocalVariables|GetVarCustomVariablesPrivate))))

(fn AddCustomVariablestoPlayer
  (params (UniqueID :type Name))
  (bind (_global _private) (CallFunction|GetCustomVariables))
  (for _array_element (Utilities|Struct|BreakS_ArrayOf_FName _global)
    (bind _success (Class|BPICustomVariable|GetCustomVariableValue(Message) (Game|GetGameInstance) _array_element "None"))
    (if _success
      (Class|BPICustomVariable|SetCustomVariableValue(Message) (Game|GetGameInstance) _array_element 1 true "None")
      (else
        (Class|BPICustomVariable|AddCustomVariable(Message) (Game|GetGameInstance) _array_element 1 "None"))))
  (for _array_element_2 (Utilities|Struct|BreakS_ArrayOf_FName _private)
    (bind _success_2 (Class|BPICustomVariable|GetCustomVariableValue(Message) (Game|GetGameInstance) _array_element_2 UniqueID))
    (if _success_2
      (Class|BPICustomVariable|SetCustomVariableValue(Message) (Game|GetGameInstance) _array_element_2 1 true UniqueID)
      (else
        (Class|BPICustomVariable|AddCustomVariable(Message) (Game|GetGameInstance) _array_element_2 1 UniqueID)))))

(fn GetInteractInfo
  (params (RPGSystem :type BPC%20RPG%20System%20Object%20Reference))
  (bind _worldlocation (CallFunction|GetMovetoEndDestination))
  (return (not (Variables|Default|GetOpen)) (select (< (CallFunction|GetDistanceXY (Transformation|GetActorLocation (Components|GetOwner RPGSystem)) _worldlocation) (Variables|Default|GetMinDistanceToInteract)) "NewEnumerator0" "NewEnumerator1")))

(fn GetMovetoEndDestination
  (return true (+ (Transformation|GetActorLocation) (* (Transformation|GetActorForwardVector) 1.2e+02))))

(fn GetScreenTooltipInfo
  (params (RPGSystem :type BPC%20RPG%20System%20Object%20Reference))
  (bind _action (CallFunction|GetInteractInfo RPGSystem)) ; Checking distance
  (return true (Utilities|Select :Index _action :NewEnumerator0 "Open [E]" :NewEnumerator1 "Too far away" :NewEnumerator2 "") "(R=1.000000,G=1.000000,B=1.000000,A=1.000000)"))

(fn GetWorldTooltipInfo
  (return (not (Variables|Default|GetOpen)) false "Treasure" "(R=1.000000,G=1.000000,B=1.000000,A=1.000000)" "0, 0, 0"))