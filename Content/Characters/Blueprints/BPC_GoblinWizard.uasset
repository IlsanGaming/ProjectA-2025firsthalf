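; Goblin wizard character Blueprint that attacks with a projectile and extends a parent class.
; On attack begin it plays the attack animation on the body and each separate clothing and accessory mesh, then spawns a BP_Projectile at the actor's transform after a fixed delay.
; Attack end does nothing, and death turns on physics simulation for the weapon.
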(event Custom|OnAttackBegin
  (Components|Animation|PlayAnimation (Variables|Character|GetMesh) "/Game/Characters/Goblin/Animation/Anim_Goblin_Wizard_attack_01.Anim_Goblin_Wizard_attack_01" false)
  (Utilities|FlowControl|Delay 1.5)
  (Game|SpawnActorfromClass "/Game/Characters/Blueprints/BP_Projectile.BP_Projectile_C" (Transformation|GetActorTransform) "AlwaysSpawn" "MultiplyWithRoot" 0 0))

(event Custom|OnAttackEnd)

(event Custom|GoblinDie
  (Physics|SetSimulatePhysics (Variables|Default|GetWeapon) true))

(fn ConstructionScript
  (|CallParentFunction))