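; Enemy AI controller that seeds its blackboard and starts the BT_Enemy behavior tree on possession.
; It stores the pawn's location as home, picks a random navigable point nearby as the initial roam target, and randomizes an idle time, all set only at possession.
; A debug print makes its own random-point query, so the printed location can differ from the stored target.
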(event EventPossess
  (params (PossessedPawn :type Pawn%20Object%20Reference))
  (bind _returnvalue (Pawn|GetControlledPawn))
  (bind _returnvalue_2 (Transformation|GetActorLocation _returnvalue))
  (bind _randomlocation (Class|NavigationSystemV1|GetRandomPointinNavigableRadius _returnvalue_2 1e+03 0 0))
  (Utilities|FlowControl|Sequence
    (:then_0
      (Class|AIController|UseBlackboard "/Game/Characters/Blueprints/AI/BB_EnemyBB.BB_EnemyBB")
      ;[1 1 1] Home Loc
      (AI|Components|Blackboard|SetValueasVector (Variables|Default|GetBlackboard) (Variables|Default|GetHomeLocKey) _returnvalue_2)
      ;[1 1 1] Random Roaming
      (AI|Components|Blackboard|SetValueasVector (Variables|Default|GetBlackboard) (Variables|Default|GetTargetLocKey) _randomlocation)
      ;[1 1 1] Random Wait
      (AI|Components|Blackboard|SetValueasFloat (Variables|Default|GetBlackboard) (Variables|Default|GetIdleTimeKey) (Math|Random|RandomFloatinRange 1.0 4.0))
      (Development|PrintString (Utilities|String|ToString(Vector) _randomlocation)))
    (:then_1
      (AI|RunBehaviorTree "/Game/Characters/Blueprints/AI/BT_Enemy.BT_Enemy"))))

(fn ConstructionScript)